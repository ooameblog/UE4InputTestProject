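; BP_MyActor is an actor that exposes four custom events for tank-style movement: forward, backward, turn left and turn right.
; Each event takes a DeltaTime from its caller and scales it by MoveSpeed or RotateSpeed for frame-rate-independent steps.
; Movement follows the actor's forward vector without sweeping for collision, and turns combine a yaw delta with the current rotation.
; BeginPlay, Tick, overlap and the construction script are empty.
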(event `self.MoveForward`
  (params (_deltaTime :type "Float (single-precision)"))
  (bind _returnvalue_location (`KismetMathLibrary.BreakTransform` (`self.GetTransform`)))
  ;[1 1 1] MoveForward Event
  (`self.K2_SetActorLocation` (+ (* (`KismetMathLibrary.GetForwardVector` (`self.K2_GetActorRotation`)) (* _deltaTime (`self.MoveSpeed`))) _returnvalue_location)))

(event `self.TurnRight`
  (params (_deltaTime :type "Float (single-precision)"))
  ;[1 1 1] TurnRight Event
  (`self.K2_SetActorRotation` (`KismetMathLibrary.ComposeRotators` (`self.K2_GetActorRotation`) (`KismetMathLibrary.MakeRotator` 0.0 0.0 (* _deltaTime (`self.RotateSpeed`))))))

(event `self.MoveBackward`
  (params (_deltaTime :type "Float (single-precision)"))
  (bind _returnvalue_location (`KismetMathLibrary.BreakTransform` (`self.GetTransform`)))
  ;[1 1 1] MoveBackward Event
  (`self.K2_SetActorLocation` (+ (* (`KismetMathLibrary.GetForwardVector` (`self.K2_GetActorRotation`)) (* (* _deltaTime (`self.MoveSpeed`)) -1.0)) _returnvalue_location)))

(event `self.TurnLeft`
  (params (_deltaTime :type "Float (single-precision)"))
  ;[1 1 1] TurnLeft Event
  (`self.K2_SetActorRotation` (`KismetMathLibrary.ComposeRotators` (`self.K2_GetActorRotation`) (`KismetMathLibrary.MakeRotator` 0.0 0.0 (* (* _deltaTime (`self.RotateSpeed`)) -1.0)))))

(fn `UserConstructionScript`)